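; Base Blueprint for interactable world entities that track a Restoration level and can be discovered in the player's encyclopedia.
; Interacting adds the entity's data asset to the player's encyclopedia, raises Restoration and requests saves through the game instance.
; Save, load and reset events use a save-game map keyed by data asset, then broadcast encyclopedia updates.
; Restoration drives the sphere's visuals through custom primitive data.
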(event EventBeginPlay
  (bind _self self)
  (Class|BPISaveHandler|RequestLoad(Message) (Game|GetGameInstance) _self)
  (CallFunction|UpdateEntityData _self))

(event Collision|EventActorBeginOverlap
  (params (OtherActor :type Actor%20Object%20Reference)))

(event EventTick
  (params (DeltaSeconds :type Float%20%28single-precision%29)))

(event EventInteract
  (params (InstigatorPawn :type Pawn%20Object%20Reference))
  (bind _entitydataasset (Variables|EntityProperties|GetEntityDataAsset))
  (bind _asbp_player_character (Utilities|Casting|CastToBP_PlayerCharacter InstigatorPawn))
  (if (Variables|Default|GetbIsInteractable)
    (Utilities|FlowControl|Sequence
      (:then_0
        (if (not (Utilities|Array|ContainsItem (Variables|/Game/Player/Encyclopedia/BP_EncyclopediaComponent.BP_EncyclopediaComponent_C|GetEntityIDs (Variables|/Game/Player/BP_PlayerCharacter.BP_PlayerCharacter_C|GetBP_EncyclopediaComponent _asbp_player_character)) _entitydataasset))
          (Utilities|Array|AddUnique (Variables|/Game/Player/Encyclopedia/BP_EncyclopediaComponent.BP_EncyclopediaComponent_C|GetEntityIDs (Variables|/Game/Player/BP_PlayerCharacter.BP_PlayerCharacter_C|GetBP_EncyclopediaComponent _asbp_player_character)) _entitydataasset)
          (Class|BPISaveHandler|RequestSave(Message) (Game|GetGameInstance) _asbp_player_character)))
      (:then_1
        (Class|MfEntity|ApplyRestorationChange 0.1)
        (CallFunction|UpdateEntityData))
      (:then_2
        (Class|BPISaveHandler|RequestSave(Message) (Game|GetGameInstance) self)))))

(event EventSaveData
  (params (SaveGameObject :type BP%20Save%20Game%20Object%20Reference))
  (bind _entitycontainer (Variables|/Game/Save/BP_SaveGame.BP_SaveGame_C|GetEntityContainer SaveGameObject))
  (if (Utilities|Map|Contains (Variables|/Game/Save/BP_SaveGame.BP_SaveGame_C|GetEntityContainer SaveGameObject) (Variables|EntityProperties|GetEntityDataAsset))
    (Utilities|Map|Remove (Variables|/Game/Save/BP_SaveGame.BP_SaveGame_C|GetEntityContainer SaveGameObject) (Variables|EntityProperties|GetEntityDataAsset)))
  (Utilities|Map|Add _entitycontainer (Variables|EntityProperties|GetEntityDataAsset) (Utilities|Struct|MakeS_SaveData_Entity (Variables|Default|GetRestoration)))
  (Default|CallUpdateEntityEncyclopediaData (.Value (Utilities|Map|Find _entitycontainer (Variables|EntityProperties|GetEntityDataAsset))) (Variables|EntityProperties|GetEntityDataAsset)))

(event EventLoadData
  (params (SaveGameObject :type BP%20Save%20Game%20Object%20Reference))
  (bind _entitydataasset (Variables|EntityProperties|GetEntityDataAsset))
  (bind _entitycontainer (Variables|/Game/Save/BP_SaveGame.BP_SaveGame_C|GetEntityContainer SaveGameObject))
  (bind (_value _returnvalue) (Utilities|Map|Find _entitycontainer _entitydataasset))
  (Utilities|FlowControl|Sequence
    (:then_0
      (if _returnvalue
        (Class|MfEntity|SetRestoration (Utilities|Struct|BreakS_SaveData_Entity _value))))
    (:then_1
      (Default|CallUpdateEntityEncyclopediaData _value (Variables|EntityProperties|GetEntityDataAsset)))))

(event EventResetData
  (params (SaveGameObject :type BP%20Save%20Game%20Object%20Reference))
  (bind _restoration (Utilities|GetClassDefaults "/Script/HobbyProject.MfEntity"))
  (bind _entitycontainer (Variables|/Game/Save/BP_SaveGame.BP_SaveGame_C|GetEntityContainer SaveGameObject))
  (if (Utilities|Map|Contains (Variables|/Game/Save/BP_SaveGame.BP_SaveGame_C|GetEntityContainer SaveGameObject) (Variables|EntityProperties|GetEntityDataAsset))
    (Utilities|Map|Remove (Variables|/Game/Save/BP_SaveGame.BP_SaveGame_C|GetEntityContainer SaveGameObject) (Variables|EntityProperties|GetEntityDataAsset)))
  (Utilities|Map|Add _entitycontainer (Variables|EntityProperties|GetEntityDataAsset) (Utilities|Struct|MakeS_SaveData_Entity _restoration))
  (Class|MfEntity|SetRestoration _restoration)
  (CallFunction|UpdateEntityData)
  (Default|CallUpdateEntityEncyclopediaData (.Value (Utilities|Map|Find _entitycontainer (Variables|EntityProperties|GetEntityDataAsset))) (Variables|EntityProperties|GetEntityDataAsset)))

(fn ConstructionScript)

(fn UpdateEntityData
  (Rendering|Material|SetCustomPrimitiveDataFloat (Variables|Default|GetSphere) 0 (Variables|Default|GetRestoration)))