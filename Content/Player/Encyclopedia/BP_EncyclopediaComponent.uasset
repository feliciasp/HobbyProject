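; BP_EncyclopediaComponent stores the player's encyclopedia as a collection of EntityIDs and persists it through the save game.
; Load and save events copy the IDs from and to the save object's PlayerData, and reset clears both copies.
; It has no active BeginPlay or Tick logic, and nothing in this graph adds entries.
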(event EventBeginPlay)

(event EventTick
  (params (DeltaSeconds :type Float%20%28single-precision%29)))

(event EventResetData
  (params (SaveGameObject :type BP%20Save%20Game%20Object%20Reference))
  (Utilities|Array|Clear (.entityids (Variables|/Game/Save/BP_SaveGame.BP_SaveGame_C|GetPlayerData SaveGameObject)))
  (Utilities|Array|Clear (Variables|Defaults|GetEntityIDs)))

(event EventLoadData
  (params (SaveGameObject :type BP%20Save%20Game%20Object%20Reference))
  (Variables|Defaults|SetEntityIDs (.entityids (Variables|/Game/Save/BP_SaveGame.BP_SaveGame_C|GetPlayerData SaveGameObject))))

(event EventSaveData
  (params (SaveGameObject :type BP%20Save%20Game%20Object%20Reference))
  (bind _playerdata (Variables|/Game/Save/BP_SaveGame.BP_SaveGame_C|GetPlayerData SaveGameObject))
  (Utilities|Array|Clear (.entityids _playerdata))
  (Utilities|Array|AppendArray (.entityids _playerdata) (Variables|Defaults|GetEntityIDs)))