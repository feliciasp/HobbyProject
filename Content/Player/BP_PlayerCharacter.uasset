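; Player character Blueprint that handles camera zoom, an encyclopedia screen and save data relay.
; On BeginPlay it requests a load from the GameInstance and creates a hidden encyclopedia widget, which Tab toggles along with input mode and cursor; O requests a reset.
; Save, load and reset events forward to every BPI_Saveable component, then refresh the encyclopedia data.
; Mouse wheel adjusts a clamped zoom value that interpolates spring arm length.
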(event EventBeginPlay
  (Utilities|FlowControl|Sequence
    (:then_0
      (Class|BPISaveHandler|RequestLoad(Message) (Game|GetGameInstance) self))
    (:then_1
      (Utilities|IsValid (Variables|HUD|GetEncyclopediaWidget)
        (:Is%20Not%20Valid
          (bind _returnvalue (UserInterface|CreateWidget "/Game/Widgets/UI/Encyclopedia/WBP_Encyclopedia.WBP_Encyclopedia_C" (Game|GetPlayerController 0)))
          (bind _output_get (Variables|HUD|SetEncyclopediaWidget _returnvalue))
          (UserInterface|Viewport|AddtoViewport _output_get 0)
          (Widget|SetVisibility (Variables|HUD|GetEncyclopediaWidget) "Collapsed"))))))

(event Collision|EventActorBeginOverlap
  (params (OtherActor :type Actor%20Object%20Reference)))

(event EventTick
  (params (DeltaSeconds :type Float%20%28single-precision%29)))

(event EventResetData
  (params (SaveGameObject :type BP%20Save%20Game%20Object%20Reference))
  (for _array_element (Class|Actor|GetComponentsbyInterface "/Game/Save/BPI_Saveable.BPI_Saveable_C")
    (Class|BPISaveable|ResetData(Message) _array_element SaveGameObject))
  (Default|CallUpdatePlayerEncyclopediaData (Variables|Default|GetBP_EncyclopediaComponent)))

(event EventLoadData
  (params (SaveGameObject :type BP%20Save%20Game%20Object%20Reference))
  (for _array_element (Class|Actor|GetComponentsbyInterface "/Game/Save/BPI_Saveable.BPI_Saveable_C")
    (Class|BPISaveable|LoadData(Message) _array_element SaveGameObject))
  (Default|CallUpdatePlayerEncyclopediaData (Variables|Default|GetBP_EncyclopediaComponent)))

(event EventSaveData
  (params (SaveGameObject :type BP%20Save%20Game%20Object%20Reference))
  (for _array_element (Class|Actor|GetComponentsbyInterface "/Game/Save/BPI_Saveable.BPI_Saveable_C")
    (Class|BPISaveable|SaveData(Message) _array_element SaveGameObject))
  (Default|CallUpdatePlayerEncyclopediaData (Variables|Default|GetBP_EncyclopediaComponent)))

(event Input|MouseEvents|MouseWheelUp
  (params (Key :type Key%20Structure :default "None"))
  (:Pressed
    (Variables|Camera|SetCameraZoomValue (Math|Float|Clamp(Float) (- (Variables|Camera|GetCameraZoomValue) 0.1)))
    (Camera|CameraZoom)))

(event Input|MouseEvents|MouseWheelDown
  (params (Key :type Key%20Structure :default "None"))
  (:Pressed
    (Variables|Camera|SetCameraZoomValue (Math|Float|Clamp(Float) (+ (Variables|Camera|GetCameraZoomValue) 0.1)))
    (Camera|CameraZoom)))

(event Input|KeyboardEvents|Tab
  (params (Key :type Key%20Structure :default "None"))
  (bind _returnvalue (Game|GetPlayerController 0))
  (bind _returnvalue_2 (Game|GetPlayerController 0))
  (:Pressed
    (Utilities|FlowControl|FlipFlop
      (:A
        (Utilities|FlowControl|Sequence
          (:then_0
            (Widget|SetVisibility (Variables|HUD|GetEncyclopediaWidget) "SelfHitTestInvisible"))
          (:then_1
            (Input|SetInputModeGameandUI _returnvalue (Variables|HUD|GetEncyclopediaWidget) "DoNotLock" true false)
            (Variables|/Script/Engine.PlayerController|SetbShowMouseCursor _returnvalue true))))
      (:B
        (Widget|SetVisibility (Variables|HUD|GetEncyclopediaWidget) "Collapsed")
        (Input|SetInputModeGameOnly _returnvalue_2 false)
        (Variables|/Script/Engine.PlayerController|SetbShowMouseCursor _returnvalue_2 false)))))

(event Input|KeyboardEvents|O
  (params (Key :type Key%20Structure :default "None"))
  (:Pressed
    (Class|BPISaveHandler|RequestReset(Message) (Game|GetGameInstance))))

(fn ConstructionScript)

(fn CameraZoom
  (Variables|/Script/Engine.SpringArmComponent|SetTargetArmLength (Variables|Default|GetSpringArmComp) (Math|Float|Lerp (Variables|Camera|GetCameraMinZoom) (Variables|Camera|GetCameraMaxZoom) (Variables|Camera|GetCameraZoomValue))))