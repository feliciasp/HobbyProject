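; BP_PetRock is a pet rock pickup that, on interaction, makes the player character's PetRock component visible and destroys itself.
; An overlap volume toggles a "Pick Up" prompt widget for the player.
; The picked-up state persists through save, load and reset events on the save game's PetRockData struct.
; It requests a load on BeginPlay, destroying itself if already collected, and requests a save on pickup.
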(event OnComponentBeginOverlap(InteractionVolume)
  (params (OverlappedComponent :type Primitive%20Component%20Object%20Reference) (OtherActor :type Actor%20Object%20Reference) (OtherComp :type Primitive%20Component%20Object%20Reference) (OtherBodyIndex :type Integer) (bFromSweep :type Boolean) (SweepResult :type Hit%20Result%20Structure%20%28by%20ref%29))
  ;[0.07292 0.07292 0.07292] On iteraction volume overlap
  (if (== (Utilities|GetClass OtherActor) "/Game/Player/BP_PlayerCharacter.BP_PlayerCharacter_C")
    (Rendering|SetVisibility (Variables|Default|GetInteractionWidget) true false)))

(event OnComponentEndOverlap(InteractionVolume)
  (params (OverlappedComponent :type Primitive%20Component%20Object%20Reference) (OtherActor :type Actor%20Object%20Reference) (OtherComp :type Primitive%20Component%20Object%20Reference) (OtherBodyIndex :type Integer))
  ;[0.07292 0.07292 0.07292] On iteraction volume overlap
  (if (== (Utilities|GetClass OtherActor) "/Game/Player/BP_PlayerCharacter.BP_PlayerCharacter_C")
    (Rendering|SetVisibility (Variables|Default|GetInteractionWidget) false false)))

(event EventInteract
  (params (InstigatorPawn :type Pawn%20Object%20Reference))
  (bind _asbp_player_character (Utilities|Casting|CastToBP_PlayerCharacter InstigatorPawn))
  (Rendering|SetVisibility (Variables|/Game/Player/BP_PlayerCharacter.BP_PlayerCharacter_C|GetPetRock _asbp_player_character) true false)
  (Variables|Default|SetPickedUp true)
  (Class|BPISaveHandler|RequestSave(Message) (Game|GetGameInstance) self)
  (Actor|DestroyActor self))

(event EventBeginPlay
  (Class|BPISaveHandler|RequestLoad(Message) (Game|GetGameInstance) self)
  (if (Variables|Default|GetPickedUp)
    (Actor|DestroyActor self)
    (else
      (bind _aswbp_interact_prompt (Utilities|Casting|CastToWBP_InteractPrompt (UserInterface|GetUserWidgetObject (Variables|Default|GetInteractionWidget))))
      (Variables|/Script/UMG.TextBlock|SetText (Variables|/Game/Widgets/UI/Interact/WBP_InteractPrompt.WBP_InteractPrompt_C|GetTB_InteractText _aswbp_interact_prompt) "Pick Up"))))

(event EventSaveData
  (params (SaveGameObject :type BP%20Save%20Game%20Object%20Reference))
  (Utilities|Struct|SetmembersinS_SaveData_PetRock (Variables|/Game/Save/BP_SaveGame.BP_SaveGame_C|GetPetRockData SaveGameObject) (Variables|Default|GetPickedUp)))

(event EventLoadData
  (params (SaveGameObject :type BP%20Save%20Game%20Object%20Reference))
  (Variables|Default|SetPickedUp (.PickedUp (Utilities|Struct|BreakS_SaveData_PetRock (Variables|/Game/Save/BP_SaveGame.BP_SaveGame_C|GetPetRockData SaveGameObject)))))

(event EventResetData
  (params (SaveGameObject :type BP%20Save%20Game%20Object%20Reference))
  (Utilities|Struct|SetmembersinS_SaveData_PetRock (Variables|/Game/Save/BP_SaveGame.BP_SaveGame_C|GetPetRockData SaveGameObject) false)
  (Variables|Default|SetPickedUp false))

(fn ConstructionScript)