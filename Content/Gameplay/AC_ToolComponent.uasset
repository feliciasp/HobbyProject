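; Player tool component that runs the active tool on use, currently only a fishing rod minigame.
; Casting traces down ahead of the player, locks movement and spawns a lure, then randomized timers trigger a bite and a short catch window.
; Using again cancels or catches, comparing a roll up to the summed rarities against sorted DA_Fish_CatchingTable rarities to pick a random fish from that tier.
; New catches enter the encyclopedia component and request a save.
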(event Custom|UseActiveTool
  (if (Variables|Default|GetToolInactive)
    ;[0.07812 0.07812 0.07812] If no tools is being used start using a tool
    (switch Utilities|FlowControl|Switch|SwitchonE_Tools (Variables|Default|GetActiveTool)
      (:NewEnumerator1
        (Fish|Fish)))
    (else
      ;[0.1146 0.1146 0.1146] If tool is active handle tool event
      (switch Utilities|FlowControl|Switch|SwitchonE_Tools (Variables|Default|GetActiveTool)
        (:NewEnumerator1
          (if (Variables|Fishing|GetFishToCatch)
            (Fish|FishCought)
            (else
              (Fish|RemoveOldFishingInstance false))))))))

(fn Fish
  (bind _returnvalue (Game|Player|GetPlayerPawn 0))
  (bind _throwingdistance (Variables|Fishing|GetThrowingDistance))
  (bind _returnvalue_2 (Transformation|GetActorLocation _returnvalue))
  (bind _returnvalue_3 (Transformation|GetActorForwardVector _returnvalue))
  (bind _returnvalue_4 (* _returnvalue_3 _throwingdistance))
  (bind _returnvalue_5 (+ _returnvalue_2 _returnvalue_4))
  (bind (_outhit _returnvalue_6) (Collision|LineTraceByChannel _returnvalue_5 (- _returnvalue_5 "0.000000,0.000000,1000.000000") "TraceTypeQuery3" false 0 "None"))
  (if _returnvalue_6
    (bind _asmf_character (Utilities|Casting|CastToMfCharacter (Game|GetPlayerCharacter 0)))
    (Variables|/Script/HobbyProject.MfCharacter|SetbDisableMovement _asmf_character true)
    (Utilities|FlowControl|Sequence
      (:then_0
        (Fish|RemoveOldFishingInstance true))
      (:then_1
        (bind _returnvalue_7 (Game|SpawnActorfromClass "/Game/Gameplay/Fishing/GBP_FishingLure.GBP_FishingLure_C" (Math|Transform|MakeTransform (.Location (Collision|BreakHitResult _outhit)) "0, 0, 0" "1.000000,1.000000,1.000000") "AlwaysSpawn" "MultiplyWithRoot" 0 0))
        (bind _output_get (Variables|Fishing|SetActiveFishingLure _returnvalue_7))
        (bind _returnvalue_8 (Niagara|SpawnSystematLocation "/Game/Gameplay/Fishing/VFX/NS_VFX_FishingSplash.NS_VFX_FishingSplash" (- (Transformation|GetActorLocation _output_get) "0.000000,0.000000,5.000000")))
        (Niagara|SetNiagaraVariable(Float) _returnvalue_8 "SplashAngle" 0.5)
        (Niagara|SetNiagaraVariable(Float) _returnvalue_8 "SplashVelocity" 0.8)
        (Variables|Fishing|SetFishing true)
        (Variables|Default|SetToolInactive false)
        (bind _returnvalue_9 (Utilities|Time|SetTimerbyFunctionName 0 "FishBaited" 5.0 false 0.0 5.0))
        (Variables|Fishing|SetFishBaitEventHandler _returnvalue_9)))))

(fn RemoveOldFishingInstance
  (params (disableMovement :type Boolean))
  (Utilities|FlowControl|Sequence
    (:then_0
      (Utilities|IsValid (Variables|Fishing|GetActiveFishingLure)
        (:Is%20Valid
          (Actor|DestroyActor (Variables|Fishing|GetActiveFishingLure)))))
    (:then_1
      (Utilities|Time|ClearandInvalidateTimerbyHandle (Variables|Fishing|GetFishBaitEventHandler))
      (Utilities|Time|ClearandInvalidateTimerbyHandle (Variables|Fishing|GetFishCancelEventHandler)))
    (:then_2
      (bind _asmf_character (Utilities|Casting|CastToMfCharacter (Game|GetPlayerCharacter 0)))
      (Variables|/Script/HobbyProject.MfCharacter|SetbDisableMovement _asmf_character disableMovement))
    (:then_3
      (Variables|Fishing|SetFishing false)
      (Variables|Default|SetToolInactive true))))

(fn FishBaited
  (bind _activefishinglure (Variables|Fishing|GetActiveFishingLure))
  (Utilities|IsValid _activefishinglure
    (:Is%20Valid
      (Niagara|SpawnSystematLocation "/Game/Gameplay/Fishing/VFX/NS_VFX_FishingSplash.NS_VFX_FishingSplash" (- (Transformation|GetActorLocation _activefishinglure) "0.000000,0.000000,5.000000"))
      (Transformation|AddLocalOffset (Variables|/Game/Gameplay/Fishing/GBP_FishingLure.GBP_FishingLure_C|GetLure _activefishinglure) "0.000000,0.000000,-15.000000" false false)
      (Utilities|FlowControl|Sequence
        (:then_0
          (Rendering|SetVisibility (Variables|/Game/Gameplay/Fishing/GBP_FishingLure.GBP_FishingLure_C|GetExclamationMark (Variables|Fishing|GetActiveFishingLure)) true false)
          (Variables|Fishing|SetFishToCatch true))
        (:then_1
          (bind _returnvalue (Utilities|Time|SetTimerbyEvent (EventDispatchers|CreateEvent :!event CancelFish) 2.0 false 0.0 0.5))
          (Variables|Fishing|SetFishCancelEventHandler _returnvalue))))))

(fn CancelFish
  (Variables|Fishing|SetFishToCatch false)
  (Fish|RemoveOldFishingInstance false))

(fn FishCought
  (bind _returnvalue (Game|GetPlayerCharacter 0))
  (bind _returnvalue_2 (Actor|GetComponentbyClass _returnvalue "/Game/Player/Encyclopedia/BP_EncyclopediaComponent.BP_EncyclopediaComponent_C"))
  (bind _fishid (Variables|/Game/Player/Encyclopedia/BP_EncyclopediaComponent.BP_EncyclopediaComponent_C|GetFishID _returnvalue_2))
  (Utilities|FlowControl|Sequence
    (:then_0
      (bind (_sum _possiblevalues) (Fish|GetFishSumOdds))
      (bind _fish (Fish|GetWeightedCatch (Math|Random|RandomFloatinRange 0.0 _sum) _possiblevalues))
      (Development|PrintString (Utilities|String|ToString(Text) (Variables|/Game/Gameplay/Fishing/PDA_Fish.PDA_Fish_C|GetSpecies _fish)))
      (if (== (Utilities|Array|FindItem _fishid _fish) -1)
        ;[0.05729 0.05729 0.05729] Updating fish data and requesting save from player
        ; Maybe encyclopedia comp should call save for this. Feels a little messy to go through player when the comp hold the data
        (Utilities|Array|AddUnique _fishid _fish)
        (Class|BPISaveHandler|RequestSave(Message) (Game|GetGameInstance) _returnvalue)))
    (:then_1
      (Fish|CancelFish))))

(fn GetFishSumOdds
  (LocalVariables|Set_sum 0.0)
  (Utilities|Array|Clear (LocalVariables|Get_possibleValues))
  (bind _outrownames (DataTable|GetDataTableRowNames "/Game/Gameplay/Fishing/DA_Fish_CatchingTable.DA_Fish_CatchingTable"))
  (for _array_element _outrownames
    (bind _returnvalue (Utilities|GetDataTableRow "/Game/Gameplay/Fishing/DA_Fish_CatchingTable.DA_Fish_CatchingTable" _array_element)
      (:then
        (LocalVariables|Set_sum (+ (.Rarity (Utilities|Struct|BreakS_Fish_CatchingTableRow _returnvalue)) (LocalVariables|Get_sum)))
        (Utilities|Array|Add (LocalVariables|Get_possibleValues) (Math|Conversions|ToFloat(Integer) (.Rarity (Utilities|Struct|BreakS_Fish_CatchingTableRow _returnvalue)))))))
  (return (LocalVariables|Get_sum) (LocalVariables|Get_possibleValues)))

(fn GetWeightedCatch
  (params (RandomValue :type Float%20%28double-precision%29) (PossibleValues :type Array%20of%20Floats%20%28double-precision%29))
  (LocalVariables|Set_rarity (.MaxValue (Math|Float|MaxOfFloatArray PossibleValues)))
  (LocalVariables|Set_fish 0)
  (bind _sorted (CallFunction|SortbySmallestNumber PossibleValues))
  (bind _array_element (Utilities|Array|ForEachLoopwithBreak _sorted :!label _label)
    (:LoopBody
      (if (<= RandomValue _array_element)
        (LocalVariables|Set_rarity _array_element)
        (goto _label Break)))
    (:Completed
      (bind _outrownames (DataTable|GetDataTableRowNames "/Game/Gameplay/Fishing/DA_Fish_CatchingTable.DA_Fish_CatchingTable"))
      (bind _array_element_2 (Utilities|Array|ForEachLoopwithBreak _outrownames)
        (:LoopBody
          (bind _returnvalue (Utilities|GetDataTableRow "/Game/Gameplay/Fishing/DA_Fish_CatchingTable.DA_Fish_CatchingTable" _array_element_2)
            (:then
              (if (== (.Rarity (Utilities|Struct|BreakS_Fish_CatchingTableRow _returnvalue)) (LocalVariables|Get_rarity))
                (LocalVariables|Set_fish (.OutItem (Utilities|Array|Random (.Fish (Utilities|Struct|BreakS_Fish_CatchingTableRow _returnvalue)))))))))
        (:Completed
          (return (LocalVariables|Get_fish)))))))