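; BP_SaveGame is a save game object that brokers saving, loading and resetting of data for saveable objects.
; It holds no data logic in these functions, instead passing itself through message calls so each object handles its own state.
; SaveData forwards to the supplied objects, LoadData answers a single requester, and ResetData loops over an array of objects.
; No disk or slot operations appear here.
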(fn SaveData
  (params (SaveableObjects :type Object%20Object%20Reference))
  (Class|BPISaveable|SaveData(Message) SaveableObjects self)
  (return))

(fn LoadData
  (params (Requester :type Object%20Object%20Reference))
  (Class|BPISaveable|LoadData(Message) Requester self)
  (return))

(fn ResetData
  (params (SaveableObjects :type Array%20of%20Object%20Object%20References))
  (for _array_element SaveableObjects
    (Class|BPISaveable|ResetData(Message) _array_element self))
  (return))